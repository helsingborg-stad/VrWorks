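; BP_VRButton is a physical VR push button that a motion controller presses, glowing when fully depressed.
; Overlapping a BP_MotionController starts tracking and stores the controller and button start locations.
; Each tick projects controller movement onto the button's up vector, using its clamped magnitude, regardless of direction, to sink the mesh.
; Maximum travel sets Glow on a dynamic material; nothing stops tracking or resets the button.
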(event `self.ReceiveBeginPlay`
  (bind _returnvalue (`PrimitiveComponent.CreateDynamicMaterialInstance` (`self.VR_Button`) 0 "/Game/UI/Button.Button" "None"))
  (set `self.MI Button` _returnvalue))

(event `self.VR_Button.OnComponentBeginOverlap`
  (params (OverlappedComponent :type "PrimitiveComponent Object Reference") (OtherActor :type "Actor Object Reference") (OtherComp :type "PrimitiveComponent Object Reference") (OtherBodyIndex :type Integer) (bFromSweep :type Boolean) (SweepResult :type "HitResult Structure (by ref)"))
  (bind _asbp_motion_controller (cast `/Game/VirtualRealityBP/Blueprints/BP_MotionController` OtherActor))
  (set `self.Tracking MC` (`/Game/VirtualRealityBP/Blueprints/BP_MotionController.MotionController` _asbp_motion_controller))
  (set `self.bIsTracking` true)
  (set `self.MC Initial Location` (`SceneComponent.K2_GetComponentLocation` (`self.Tracking MC`)))
  (set `self.Button Initial Location` (`SceneComponent.K2_GetComponentLocation` (`self.VR_Button`))))

(event `self.ReceiveTick`
  (params (DeltaSeconds :type "Float (single-precision)"))
  (bind _vr_button (`self.VR_Button`))
  (if (`self.bIsTracking`)
    (set `self.Current Travel` (`KismetMathLibrary.FClamp` (`KismetMathLibrary.Abs` (`KismetMathLibrary.VSize` (`KismetMathLibrary.ProjectVectorOnToVector` (- (`SceneComponent.K2_GetComponentLocation` (`self.Tracking MC`)) (`self.MC Initial Location`)) (`SceneComponent.GetUpVector` (`self.VR_Button`))))) 0.0 (`self.Maximum Travel`)))
    (bind _output_get (set `self.Button Current Location` (- (`self.Button Initial Location`) (* (`SceneComponent.GetUpVector` _vr_button) (`self.Current Travel`)))))
    (`SceneComponent.K2_SetWorldLocation` _vr_button _output_get false false)
    (if (>= (`self.Current Travel`) (`self.Maximum Travel`))
      (`self.Fully Pressed`))))

(event `Fully Pressed`
  (`MaterialInstanceDynamic.SetScalarParameterValue` (`self.MI Button`) "Glow" (`self.Glow Intensity`)))

(fn `UserConstructionScript`)